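; Player controller for the Push game mode that handles player list registration and a key-triggered resource increase.
; Shortly after BeginPlay, it asks PushGameMode, when valid, to update its player list.
; Pressing F chains a server event into an event named as a multicast (NMC), which calls the ResourceComponent's server functions to adjust both gold and kills by fixed amounts.
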(event Custom|Increase%20Gold_Server
  (CallFunction|IncreaseGoldNMC))

(event Custom|Increase%20Gold_NMC
  (bind _resourcecomponent (Variables|Default|GetresourceComponent)
    (:then
      (Utilities|FlowControl|Sequence
        (:then_0
          (Class|ResourceComponent|AdjustGoldServer _resourcecomponent 1))
        (:then_1
          (Class|ResourceComponent|AdjustKillServer _resourcecomponent 2))))
    (:else)))

(event EventBeginPlay
  (bind _pushgamemode (Variables|Default|GetPushGameMode))
  (|CallParentFunction)
  (Utilities|FlowControl|Delay 0.2)
  (Utilities|IsValid _pushgamemode
    (:Is%20Valid
      (Class|PushGameMode|UpdatePlayerList _pushgamemode))))

(event Input|KeyboardEvents|F
  (params (Key :type Key%20Structure :default "None"))
  (:Pressed
    (CallFunction|IncreaseGoldServer)))

(fn ConstructionScript)