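; Test lobby game state that starts a match countdown once at least three players are connected.
; The connection notify event records the player count and, guarded by a DoOnce, sets the countdown.
; The countdown's OnRep refreshes all WDG_LobbyCountDown widgets and calls a one-second delayed decrement, forming a self-driving RepNotify loop.
; At zero it only prints a started-match message; no travel or match logic runs.
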(event Custom|Match_CountDown
  (Utilities|FlowControl|Delay 1.0)
  (Variables|Default|SetMatchStart_Countdown (- (Variables|Default|GetMatchStart_Countdown) 1)))

(event Custom|_NotifyPlayerConnection
  (bind _playerarray (Variables|Default|GetPlayerArray))
  (bind _returnvalue (Utilities|Array|Length _playerarray))
  (Variables|Default|SetCurrentAmountOfPlayers _returnvalue)
  (if (>= _returnvalue 3)
    (Utilities|FlowControl|DoOnce false
      (:Completed
        (Variables|Default|SetMatchStart_Countdown 5)))))

(fn ConstructionScript)

(fn UpdateMatchStartCoundownWidget
  (bind _foundwidgets (Widget|GetAllWidgetsOfClass "/Game/BP/Widgets/WDG_LobbyCountDown.WDG_LobbyCountDown_C" false))
  (for _array_element _foundwidgets
    (Default|UpdateWidget _array_element (Variables|Default|GetMatchStart_Countdown))))

(fn OnRepMatchStartCountdown
  (CallFunction|UpdateMatchStartCoundownWidget)
  (if (== (Variables|Default|GetMatchStart_Countdown) 5)
    (CallFunction|MatchCountDown)
    (elif (== (Variables|Default|GetMatchStart_Countdown) 0)
      (Development|PrintString "Started Match!!!!" true true "(R=0.000000,G=0.660000,B=1.000000,A=1.000000)" 3.0)
      (else
        (CallFunction|MatchCountDown)))))