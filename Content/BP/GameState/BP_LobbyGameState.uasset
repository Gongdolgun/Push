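; Lobby game state that holds a replicated match-start countdown, which the Connection event sets to 15.
; Its RepNotify pushes each new value to every WDG_LobbyCountDown widget, then calls Match_CountDown to decrement it, forming a self-driving chain with no delay shown.
; At zero the chain stops and prints a placeholder "Hello!!!" message, with no match-start logic.
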(event Custom|Match_CountDown
  (Variables|Default|SetMatchStart_Countdown (- (Variables|Default|GetMatchStart_Countdown) 1)))

(event Custom|Connection
  (Variables|Default|SetMatchStart_Countdown 15))

(fn ConstructionScript)

(fn OnRepMatchStartCountdown
  (CallFunction|UpdateMatchStartCoundownWidget)
  (if (== (Variables|Default|GetMatchStart_Countdown) 15)
    (CallFunction|MatchCountDown)
    (elif (== (Variables|Default|GetMatchStart_Countdown) 0)
      (Development|PrintString "Hello!!!" true true "(R=0.000000,G=0.660000,B=1.000000,A=1.000000)" 3.0)
      (else
        (CallFunction|MatchCountDown)))))

(fn UpdateMatchStartCoundownWidget
  (bind _foundwidgets (Widget|GetAllWidgetsOfClass "/Game/BP/Widgets/WDG_LobbyCountDown.WDG_LobbyCountDown_C" false))
  (for _array_element _foundwidgets
    (Default|UpdateWidget _array_element (Variables|Default|GetMatchStart_Countdown))))