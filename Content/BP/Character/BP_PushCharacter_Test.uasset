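; BP_PushCharacter_Test is a character Blueprint, named as a test variant, that binds player input to a shop and skill-slot system.
; On BeginPlay it shows the mouse cursor, and the B key opens the store UI through ShopComponent.
; Four Skill input actions and the Q and E keys cast ShopComponent.SkillSlots to WDG_SkillSlots, then trigger a skill or item by slot index, leaving the use logic to that widget.
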(event EventBeginPlay
  (Variables|/Script/Engine.PlayerController|SetbShowMouseCursor (Game|GetPlayerController 0) true))

(event Input|KeyboardEvents|B
  (params (Key :type Key%20Structure :default "None"))
  (:Pressed
    (Class|ShopComponent|OpenStoreUI (Variables|Default|GetShopComponent))))

(event Input|ActionEvents|InputActionSkill1
  (params (Key :type Key%20Structure))
  (:Pressed
    (bind _aswdg_skill_slots (Utilities|Casting|CastToWDG_SkillSlots (Variables|/Script/Push.ShopComponent|GetSkillSlots (Variables|Default|GetShopComponent))))
    (Default|UseSkill _aswdg_skill_slots)))

(event Input|ActionEvents|InputActionSkill2
  (params (Key :type Key%20Structure))
  (:Pressed
    (bind _aswdg_skill_slots (Utilities|Casting|CastToWDG_SkillSlots (Variables|/Script/Push.ShopComponent|GetSkillSlots (Variables|Default|GetShopComponent))))
    (Default|UseSkill _aswdg_skill_slots 1)))

(event Input|ActionEvents|InputActionSkill3
  (params (Key :type Key%20Structure))
  (:Pressed
    (bind _aswdg_skill_slots (Utilities|Casting|CastToWDG_SkillSlots (Variables|/Script/Push.ShopComponent|GetSkillSlots (Variables|Default|GetShopComponent))))
    (Default|UseSkill _aswdg_skill_slots 2)))

(event Input|ActionEvents|InputActionSkill4
  (params (Key :type Key%20Structure))
  (:Pressed
    (bind _aswdg_skill_slots (Utilities|Casting|CastToWDG_SkillSlots (Variables|/Script/Push.ShopComponent|GetSkillSlots (Variables|Default|GetShopComponent))))
    (Default|UseSkill _aswdg_skill_slots 3)))

(event Input|KeyboardEvents|Q
  (params (Key :type Key%20Structure))
  (:Pressed
    (bind _aswdg_skill_slots (Utilities|Casting|CastToWDG_SkillSlots (Variables|/Script/Push.ShopComponent|GetSkillSlots (Variables|Default|GetShopComponent))))
    (Default|UseItem _aswdg_skill_slots)))

(event Input|KeyboardEvents|E
  (params (Key :type Key%20Structure))
  (:Pressed
    (bind _aswdg_skill_slots (Utilities|Casting|CastToWDG_SkillSlots (Variables|/Script/Push.ShopComponent|GetSkillSlots (Variables|Default|GetShopComponent))))
    (Default|UseItem _aswdg_skill_slots 1)))

(fn ConstructionScript)