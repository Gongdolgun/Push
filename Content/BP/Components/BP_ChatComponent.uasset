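; BP_ChatComponent is a player controller component that provides in-game multiplayer text chat.
; On BeginPlay it creates the WDG_ChatUI widget for the local controller and keeps a reference to its chat box.
; SendChatMessage_Server relays a message through the game mode's AllPC list to each controller's chat component, whose AddChatMessageOnOwningClient appends it to the chat box.
; Input events focus or scroll the chat box.
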(event Custom|Input_Enter
  ;[1 1 1] Input Event
  (Class|ChatBox|FocusChat (Variables|Default|GetChatBox_Ref)))

(event Custom|Input_MouseDown
  ;[1 1 1] Input Event
  (Class|ChatBox|Scroll (Variables|Default|GetChatBox_Ref) false))

(event Custom|Input_MouseUp
  ;[1 1 1] Input Event
  (Class|ChatBox|Scroll (Variables|Default|GetChatBox_Ref) true))

(event Custom|SendChatMessage_Server
  (params (InMessage :type String))
  (bind _aspush_game_mode (Utilities|Casting|CastToPushGameMode (Game|GetGameMode)))
  (for _array_element (Variables|/Script/Push.PushGameMode|GetAllPC _aspush_game_mode)
    (bind _asbp_push_player_controller (Utilities|Casting|CastToBP_PushPlayerController _array_element))
    (CallFunction|AddChatMessageonOwningClient (Actor|GetComponentbyClass _asbp_push_player_controller "BP_ChatComponent_C") InMessage)))

(event Custom|AddChatMessageOnOwningClient
  (params (InMessage :type String))
  (Class|ChatBox|AddChatMessage (Variables|Default|GetChatBox_Ref) InMessage))

(event EventBeginPlay
  (bind _aspush_player_controller (Utilities|Casting|CastToPushPlayerController (Components|GetOwner)))
  (if (Pawn|IsLocalPlayerController _aspush_player_controller)
    (bind _returnvalue (UserInterface|CreateWidget "/Game/BP/Widgets/Chatting/WDG_ChatUI.WDG_ChatUI_C"))
    (bind _output_get (Variables|Default|SetChatUI_Ref _returnvalue))
    (UserInterface|Viewport|AddtoViewport _output_get 0)
    (Variables|Default|SetChatBox_Ref (Variables|/Game/BP/Widgets/Chatting/WDG_ChatUI.WDG_ChatUI_C|GetWDG_ChatBox _output_get))))